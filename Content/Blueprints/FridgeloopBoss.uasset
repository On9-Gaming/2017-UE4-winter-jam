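; FridgeloopBoss is a Blueprint that closes a gate for what its name suggests is a fridge boss area.
; On Hit, it waits half a second, then checks whether the pork player character is falling, printing debug text either way.
; If the player is grounded, a DoOnce triggers CloseGate, whose timeline slides the Gate's relative X position.
; BeginPlay caches the game state, which is otherwise unused here.
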(event `self.ReceiveBeginPlay`
  ;[1 1 1] Event BeginPlay
  (bind _asmygamestate (cast `/Game/mygamestate` (`GameplayStatics.GetGameState`)))
  (set `self.my game state` _asmygamestate))

(event `self.ReceiveHit`
  (params (MyComp :type "PrimitiveComponent Object Reference") (Other :type "Actor Object Reference") (OtherComp :type "PrimitiveComponent Object Reference") (bSelfMoved :type Boolean) (HitLocation :type "Vector Structure") (HitNormal :type "Vector Structure") (NormalImpulse :type "Vector Structure") (Hit :type "HitResult Structure (by ref)"))
  (bind _aspork (cast `/Game/Blueprints/pork` (`GameplayStatics.GetPlayerCharacter` 0)))
  (`KismetSystemLibrary.Delay` 0.5)
  (if (`NavMovementComponent.IsFalling` (`Character.CharacterMovement` _aspork))
    (`KismetSystemLibrary.PrintString` "not ready")
    (else
      (`KismetSystemLibrary.PrintString` "ready")
      (`/Engine/EditorBlueprintResources/StandardMacros.DoOnce` false
        (:`Completed`
          (`self.Close gate`))))))

(event `Close gate`
  (bind (_direction _newtrack_0) (`Timeline|close gate time line` :!via `PlayFromStart`)
    (:`Update`
      (`SceneComponent.K2_SetRelativeLocation` (`self.gate`) (`KismetMathLibrary.MakeVector` _newtrack_0 0.0 200.0) false false))))

(fn `UserConstructionScript`
  (`|ExecutionSequence`))