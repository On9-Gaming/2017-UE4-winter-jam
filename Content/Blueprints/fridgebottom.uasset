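; Fridge bottom actor that moves vertically when the game starts, then removes itself.
; BeginPlay caches the custom game state, and Tick polls its Gamestart flag behind a DoOnce.
; Once triggered, a timeline drives the absolute world Z with X and Y fixed at zero, and the actor is destroyed when it finishes.
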(event `self.ReceiveBeginPlay`
  (bind _asmygamestate (cast `/Game/mygamestate` (`GameplayStatics.GetGameState`)))
  (set `self.my game statte` _asmygamestate))

(event `self.ReceiveTick`
  (params (DeltaSeconds :type "Float (single-precision)"))
  (if (`/Game/mygamestate.gamestart?` (`self.my game statte`))
    (`/Engine/EditorBlueprintResources/StandardMacros.DoOnce` false
      (:`Completed`
        (bind (_direction _time) (`Timeline|time`)
          (:`Update`
            (`self.K2_SetActorLocation` (`KismetMathLibrary.MakeVector` 0.0 0.0 _time)))
          (:`Finished`
            (`self.K2_DestroyActor`)))))))

(fn `UserConstructionScript`)